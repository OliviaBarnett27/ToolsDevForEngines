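; PCG Blueprint element that reads the current weather and time settings from the weather selector subsystem.
; ExecuteWithContext copies climate, season, day/night, audio, erraticism and day length from the subsystem into its own variables.
; It returns without building any output data, and the node that would set members in the PCG context is not wired to run.
; Execute only forwards to the parent implementation.
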(fn Execute
  (params (Input :type PCG%20Data%20Collection%20Structure%20%28by%20ref%29))
  (bind _output (|CallParentFunction Input))
  (return _output))

(fn ExecutewithContext
  (params (InContext :type PCG%20Context%20Structure%20%28by%20ref%29) (Input :type PCG%20Data%20Collection%20Structure%20%28by%20ref%29))
  (bind _returnvalue (Subsystems|GetSubsystemWeatherSelector))
  (Variables|Default|SetClimate (Class|SubsystemWeatherSelector|GetClimate _returnvalue))
  (Variables|Default|SetSeason (Class|SubsystemWeatherSelector|GetSeason _returnvalue))
  (Variables|Default|SetDayNight (Class|SubsystemWeatherSelector|GetDayNight _returnvalue))
  (Variables|Default|SetAudio (Class|SubsystemWeatherSelector|GetAudio _returnvalue))
  (Variables|Default|SetErraticism (Class|SubsystemWeatherSelector|GetErraticism _returnvalue))
  (Variables|Default|SetDayLength (Class|SubsystemWeatherSelector|GetDayLength _returnvalue))
  (return ""))